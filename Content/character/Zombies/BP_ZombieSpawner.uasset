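; BP_ZombieSpawner spawns BP_Base_Zombie AI pawns at its own location and rotation.
; BeginPlay starts a looping half-second timer that spawns a zombie, adds it to the Zombies array and increments the spawned count.
; The max check follows the spawn, so the call that clears the timer leaves one extra, untracked zombie.
; Tick prints the array length as a debug readout.
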(event `self.ReceiveBeginPlay`
  (bind _returnvalue (`KismetSystemLibrary.K2_SetTimerDelegate` (delegate `CustomEvent`) 0.5 true true))
  (set `self.Spanw timer` _returnvalue))

(event `CustomEvent`
  (bind _zombiespawnedcount (`self.ZombieSpawnedCount`))
  (bind _returnvalue (`AIBlueprintHelperLibrary.SpawnAIFromClass` "/Game/character/Zombies/BP_Base_Zombie.BP_Base_Zombie_C" null (`self.K2_GetActorLocation`) (`self.K2_GetActorRotation`) false null))
  (bind _asbp_base_zombie (cast `/Game/character/Zombies/BP_Base_Zombie` _returnvalue))
  (if (>= _zombiespawnedcount (`self.ZombieSpawnMax`))
    (`KismetSystemLibrary.K2_ClearAndInvalidateTimerHandle` (`self.Spanw timer`))
    (else
      (`/Engine/EditorBlueprintResources/StandardMacros.IncrementInt` _zombiespawnedcount
        (:`  `
          (`KismetArrayLibrary.Array_Add` (`self.Zombies`) _asbp_base_zombie))))))

(event `self.ReceiveTick`
  (params (DeltaSeconds :type "Float (single-precision)"))
  (`KismetSystemLibrary.PrintString` (`KismetStringLibrary.Concat_StrStr` "Zombies count: " (`KismetStringLibrary.Conv_IntToString` (`KismetArrayLibrary.Array_Length` (`self.Zombies`)))) true true (struct :`R` 0.792078 :`B` 1.0 :`A` 1.0) 20.0 "Zombies"))

(fn `UserConstructionScript`)