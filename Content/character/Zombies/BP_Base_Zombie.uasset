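; BP_Base_Zombie is a zombie character blueprint that chases pawns it sees and reacts to where projectiles hit it.
; When PawnSensing sees a pawn, AI Move To sends the zombie toward it, with debug prints for each outcome that have screen output turned off.
; A ZombieHitByProjectile event switches on the body part hit: a leg hit sets a new walk speed and a head hit destroys the zombie.
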(event `self.PawnSensing.OnSeePawn`
  (params (Pawn :type "Pawn Object Reference"))
  (`|AIMoveTo` self (`self.K2_GetActorLocation` Pawn) Pawn 10.0
    (:`then`
      (`KismetSystemLibrary.PrintString` "MOVING" false true (struct :`G` 0.66 :`B` 1.0 :`A` 1.0) 2.0 "moving"))
    (:`OnSuccess`
      (`KismetSystemLibrary.PrintString` "SUCCESS" false true (struct :`G` 0.66 :`B` 1.0 :`A` 1.0) 2.0 "moving"))
    (:`OnFail`
      (`KismetSystemLibrary.PrintString` "FAIL" false true (struct :`G` 0.66 :`B` 1.0 :`A` 1.0) 2.0 "moving"))))

(event `self.PawnSensing.OnHearNoise`
  (params (Instigator :type "Pawn Object Reference") (Location :type "Vector Structure (by ref)") (Volume :type "Float (single-precision)")))

(event `ZombieHitByProjectile`
  (params (`Body Part Hit` :type "/Game/Enums/E_BodyParts Enum" :default "NewEnumerator0"))
  (switch `/Game/Enums/E_BodyParts` `Body Part Hit`
    (:`NewEnumerator1`
      (set `CharacterMovementComponent.MaxWalkSpeed` 200.0 (`self.CharacterMovement`)))
    (:`NewEnumerator2`
      (`self.K2_DestroyActor`))))

(fn `UserConstructionScript`)