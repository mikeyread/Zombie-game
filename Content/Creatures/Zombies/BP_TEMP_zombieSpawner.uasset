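; BP_TEMP_zombieSpawner is a temporary spawner actor that spawns BP_TEMP_Zombie AI pawns in the level.
; BeginPlay starts a looping half-second timer, which appears to drive Test to spawn a zombie, increment Count and pause the timer upon reaching SpawnCount.
; SpawnZombie places each pawn slightly below the spawner with a fixed rotation.
; Zombie-manager lookup and player-FPS throttling logic are present but never run.
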(event `self.ReceiveBeginPlay`
  (bind _returnvalue (`KismetSystemLibrary.K2_SetTimerDelegate` (`|CreateDelegate` :!event `Test`) 0.5 true true))
  (set `self.NewVar` _returnvalue))

(event `Test`
  (`self.SpawnZombie` "/Game/Creatures/Zombies/BP_TEMP_Zombie.BP_TEMP_Zombie_C")
  (bind _result (`/Engine/EditorBlueprintResources/StandardMacros.IncrementInt` (`self.count`))
    (:`  `
      (if (== _result (`self.Spawn count`))
        (`KismetSystemLibrary.K2_PauseTimerHandle` (`self.NewVar`))))))

(event `SpawnZombie`
  (params (Zombie :type "Pawn Class Reference"))
  (bind _returnvalue_location (`KismetMathLibrary.BreakTransform` (`self.GetTransform`)))
  (`AIBlueprintHelperLibrary.SpawnAIFromClass` Zombie null (+ _returnvalue_location (0.0 0.0 -50.0)) (struct :`Yaw` -90.0) false null))

(fn `UserConstructionScript`)