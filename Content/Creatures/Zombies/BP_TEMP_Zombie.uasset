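; Temporary zombie enemy that roams the map, chases what it senses and damages the first-person player.
; It loops AI moves to random reachable points, redirecting toward seen pawns or noise instigators via PawnSensing and resuming roaming when a chase fails.
; Capsule overlap runs a looping timer that drains player HP and notifies the game mode at zero; leaving clears it.
; A Setdead event hides the zombie and disables its collision and tick.
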(event `Set dead`
  (`self.SetActorEnableCollision` false)
  (`self.SetActorHiddenInGame` true)
  (`self.SetActorTickEnabled` false))

(event `self.ReceiveBeginPlay`
  (`KismetSystemLibrary.Delay` 5.0)
  (`self.Random roam`))

(event `self.PawnSensing.OnHearNoise`
  (params (Instigator :type "Pawn Object Reference") (Location :type "Vector Structure (by ref)") (Volume :type "Float (single-precision)"))
  (`|AIMoveTo` self (0.0 0.0 0.0) Instigator
    (:`OnFail`
      (`self.Random roam`))))

(event `self.PawnSensing.OnSeePawn`
  (params (Pawn :type "Pawn Object Reference"))
  (`|AIMoveTo` self (0.0 0.0 0.0) Pawn
    (:`OnFail`
      (`self.Random roam`))))

(event `Random roam`
  (`|AIMoveTo` self (`NavigationSystemV1.K2_GetRandomReachablePointInRadius` (`self.K2_GetActorLocation`) 25000.0 null null) null
    (:`OnSuccess`
      (`self.Random roam`))
    (:`OnFail`
      (`self.Random roam`))))

(event `self.Capsule.OnComponentBeginOverlap`
  (params (OverlappedComponent :type "PrimitiveComponent Object Reference") (OtherActor :type "Actor Object Reference") (OtherComp :type "PrimitiveComponent Object Reference") (OtherBodyIndex :type Integer) (bFromSweep :type Boolean) (SweepResult :type "HitResult Structure (by ref)"))
  (if (== (`GameplayStatics.GetObjectClass` OtherActor) "/Game/FirstPerson/Blueprints/BP_FirstPersonCharacter.BP_FirstPersonCharacter_C")
    (`KismetSystemLibrary.PrintString` "in range of player")
    (bind _returnvalue (`KismetSystemLibrary.K2_SetTimerDelegate` (delegate `CustomEvent`) 1.0 true true))
    (set `self.NewVar` _returnvalue)))

(event `CustomEvent`
  (bind _asbp_first_person_character (cast `/Game/FirstPerson/Blueprints/BP_FirstPersonCharacter` (stale `self.Capsule.OnComponentBeginOverlap` OtherActor)))
  (bind _output_get (set `/Game/FirstPerson/Blueprints/BP_FirstPersonCharacter.HP` (- (`/Game/FirstPerson/Blueprints/BP_FirstPersonCharacter.HP` _asbp_first_person_character) 10.0) _asbp_first_person_character))
  (if (> _output_get 0.0)
    (`KismetSystemLibrary.PrintString` (`KismetStringLibrary.Concat_StrStr` (`KismetSystemLibrary.GetClassDisplayName` (`GameplayStatics.GetObjectClass` self)) " hit " (`KismetSystemLibrary.GetDisplayName` (stale `self.Capsule.OnComponentBeginOverlap` OtherActor)) " health left " (`KismetStringLibrary.Conv_DoubleToString` _output_get)))
    (else
      (bind _asbp_first_person_game_mode (cast `/Game/FirstPerson/Blueprints/BP_FirstPersonGameMode` (`GameplayStatics.GetGameMode`)))
      (`/Game/FirstPerson/Blueprints/BP_FirstPersonGameMode.player killed` _asbp_first_person_game_mode _asbp_first_person_character)
      (`self.Random roam`))))

(event `self.Capsule.OnComponentEndOverlap`
  (params (OverlappedComponent :type "PrimitiveComponent Object Reference") (OtherActor :type "Actor Object Reference") (OtherComp :type "PrimitiveComponent Object Reference") (OtherBodyIndex :type Integer))
  (if (== (`GameplayStatics.GetObjectClass` OtherActor) "/Game/FirstPerson/Blueprints/BP_FirstPersonCharacter.BP_FirstPersonCharacter_C")
    (`KismetSystemLibrary.K2_ClearAndInvalidateTimerHandle` (`self.NewVar`))))

(fn `UserConstructionScript`)