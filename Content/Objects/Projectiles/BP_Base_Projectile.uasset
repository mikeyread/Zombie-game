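; Base projectile Blueprint that reports hits on zombie body parts.
; On static mesh hit, it checks for an exact base player or zombie class, but only zombies get past the cast.
; The hit component's name (Head, Body or Legs) selects the enum passed to ZombieHitByProjectile, then the projectile destroys itself.
; Other hits leave it alive, mostly printing debug text; its forward AddForce logic is unconnected.
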(event `self.ReceiveBeginPlay`)

(event `self.StaticMesh.OnComponentHit`
  (params (HitComponent :type "PrimitiveComponent Object Reference") (OtherActor :type "Actor Object Reference") (OtherComp :type "PrimitiveComponent Object Reference") (NormalImpulse :type "Vector Structure") (Hit :type "HitResult Structure (by ref)"))
  (bind _returnvalue (`KismetSystemLibrary.GetObjectName` OtherComp))
  (bind _returnvalue_2 (`GameplayStatics.GetObjectClass` OtherActor))
  (if (or (== _returnvalue_2 "/Game/character/Player/BP_Base_Player.BP_Base_Player_C") (== _returnvalue_2 "/Game/character/Zombies/BP_Base_Zombie.BP_Base_Zombie_C"))
    (`KismetSystemLibrary.PrintString` (`KismetSystemLibrary.GetDisplayName` OtherActor) true true (struct :`G` 0.66 :`B` 1.0 :`A` 1.0) 2.0 "ProjectileHit")
    (`KismetSystemLibrary.PrintString` _returnvalue true true (struct :`G` 0.66 :`B` 1.0 :`A` 1.0) 2.0 "ProjectileHit")
    (bind _asbp_base_zombie (cast `/Game/character/Zombies/BP_Base_Zombie` OtherActor))
    (switch `string` _returnvalue
      (:`Default`
        (`KismetSystemLibrary.PrintString` (`KismetStringLibrary.Concat_StrStr` "no know body part hit " _returnvalue) true true (struct :`G` 0.66 :`B` 1.0 :`A` 1.0) 2.0 "None"))
      (:`Head`
        (`/Game/character/Zombies/BP_Base_Zombie.ZombieHitByProjectile` _asbp_base_zombie "NewEnumerator2")
        (`self.K2_DestroyActor` :!label _label))
      (:`Body`
        (`/Game/character/Zombies/BP_Base_Zombie.ZombieHitByProjectile` _asbp_base_zombie "NewEnumerator0")
        (goto _label))
      (:`Legs`
        (`/Game/character/Zombies/BP_Base_Zombie.ZombieHitByProjectile` _asbp_base_zombie "NewEnumerator1")
        (goto _label)))
    (else
      (`KismetSystemLibrary.PrintString` "false" true true (struct :`G` 0.66 :`B` 1.0 :`A` 1.0) 2.0 "ProjectileHit"))))

(fn `UserConstructionScript`)